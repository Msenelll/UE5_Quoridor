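; Player controller for a Quoridor board game that sets up camera, cursor and turn-controls UI, and handles click/touch input.
; CanInteract gates input by game mode and turn, then a downward trace from the cursor hit finds the tile.
; Depending on action state, it moves the current pawn and shows end-game UI on a win, or spawns a wall on the nearest tile edge, records it in GameState and toggles turn.
; IsValidPawnMove and FindOffset helpers go uncalled here.
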(event EventTick
  (params (DeltaSeconds :type Float%20%28single-precision%29)))

(event EventBeginPlay
  ;[0.15 0.15 0.15 0.5] Preset
  (bind _asgs_quoridor (Utilities|Casting|CastToGS_Quoridor (Game|GetGameState)))
  (Variables|Default|SetGameState_Ref _asgs_quoridor)
  (bind _returnvalue (Actor|GetActorOfClass "/Script/Engine.CameraActor"))
  (Game|Player|SetViewTargetwithBlend _returnvalue 0.0 "VTBlend_Linear" 0.0 false)
  (Variables|Default|SetbShowMouseCursor true)
  (Input|SetInputModeGameOnly self false)
  (bind _returnvalue_2 (UserInterface|CreateWidget "/Game/02_Blueprint/03_UI/WBP_TurnControls.WBP_TurnControls_C"))
  (UserInterface|Viewport|AddtoViewport _returnvalue_2 0)
  (bind _returnvalue_3 (Actor|GetActorOfClass "/Game/02_Blueprint/01_Core/BP_GameBoard.BP_GameBoard_C"))
  (Variables|Default|SetGameBoard_Ref _returnvalue_3))

(event EventActorOnInputTouchBegin
  (params (FingerIndex :type ETouchIndex%20Enum :default "Touch1"))
  (bind _hitresult (Game|Player|GetHitResultUnderCursorbyChannel "TraceTypeQuery1" true))
  (bind _gamestate_ref (Variables|Default|GetGameState_Ref))
  (bind _gamestate_ref_2 (Variables|Default|GetGameState_Ref))
  (bind _gamestate_ref_3 (Variables|Default|GetGameState_Ref))
  (bind _gamestate_ref_4 (Variables|Default|GetGameState_Ref))
  (bind _gameboard_ref (Variables|Default|GetGameBoard_Ref))
  (bind _location (Collision|BreakHitResult _hitresult))
  (bind _bisplayeroneturn (Variables|/Game/02_Blueprint/01_Core/GS_Quoridor.GS_Quoridor_C|GetbIsPlayerOneTurn _gamestate_ref_3))
  (bind _gridspacing (Variables|/Game/02_Blueprint/01_Core/BP_GameBoard.BP_GameBoard_C|GetGridSpacing _gameboard_ref))
  (bind _returnvalue (/ _gridspacing 2.0))
  ;[0.15 0.15 0.15 0.5] Inputs
  ;;[0.15 0.15 0.15 0.5] TurnControl
  (bind _bcaninteract (CallFunction|CanInteract))
  (if _bcaninteract
    (bind (_outhit _returnvalue_2) (Collision|LineTraceByChannel _location (+ _location "0.000000,0.000000,-5000.000000") "TraceTypeQuery1" false 0 "None"))
    (if _returnvalue_2
      (bind _asbp_tile (Utilities|Casting|CastToBP_Tile (.HitActor (Collision|BreakHitResult _outhit))))
      (switch Utilities|FlowControl|Switch|SwitchonE_ActionState (Variables|Default|GeteCurrentActionState)
        (:NewEnumerator0
          ;[0.15 0.15 0.15 0.5] Move Pawn
          (Default|AttemptMoveto (select (Variables|/Game/02_Blueprint/01_Core/GS_Quoridor.GS_Quoridor_C|GetbIsPlayerOneTurn _gamestate_ref_4) (Variables|/Game/02_Blueprint/01_Core/GS_Quoridor.GS_Quoridor_C|GetPlayerOnePawn _gamestate_ref_4) (Variables|/Game/02_Blueprint/01_Core/GS_Quoridor.GS_Quoridor_C|GetPlayerTwoPawn _gamestate_ref_4)) (Utilities|Struct|MakeIntPoint (Variables|/Game/02_Blueprint/01_Core/BP_Tile.BP_Tile_C|GetGridX _asbp_tile) (Variables|/Game/02_Blueprint/01_Core/BP_Tile.BP_Tile_C|GetGridY _asbp_tile)) (Math|Vector|MakeVector (.x (Transformation|GetActorLocation _asbp_tile)) (.y (Transformation|GetActorLocation _asbp_tile)) (Variables|/Game/02_Blueprint/01_Core/BP_GameBoard.BP_GameBoard_C|GetPawnSpawnHeight (Variables|Default|GetGameBoard_Ref))))
          (bind _bgamehasbeenwon (Default|CheckforWinCondition _gamestate_ref_3 _bisplayeroneturn))
          (if _bgamehasbeenwon
            ;;[0.15 0.15 0.15 0.5] EndGame
            (bind _returnvalue_3 (UserInterface|CreateWidget "/Game/02_Blueprint/03_UI/WBP_EndGame.WBP_EndGame_C" 0 (|GenerictoText (select _bisplayeroneturn "Oyuncu 1 Kazandı!" "Oyuncu 2 Kazandı!"))))
            (UserInterface|Viewport|AddtoViewport _returnvalue_3 0)
            (Variables|Default|SetbShowMouseCursor true)
            (Input|SetInputModeUIOnly self _returnvalue_3 "DoNotLock" false)))
        (:NewEnumerator1
          ;[0.15 0.15 0.15 0.5] MoveWall
          (if (> (select (Variables|/Game/02_Blueprint/01_Core/GS_Quoridor.GS_Quoridor_C|GetbIsPlayerOneTurn _gamestate_ref) (Variables|/Game/02_Blueprint/01_Core/GS_Quoridor.GS_Quoridor_C|GetPlayerOneWallCount _gamestate_ref) (Variables|/Game/02_Blueprint/01_Core/GS_Quoridor.GS_Quoridor_C|GetPlayerTwoWallCount _gamestate_ref)) 0)
            (Game|SpawnActorfromClass "/Game/02_Blueprint/01_Core/BP_Wall.BP_Wall_C" (Math|Transform|MakeTransform (+ (Transformation|GetActorLocation _asbp_tile) (select (select (> (Math|Float|Absolute(Float) (.x (- (.ImpactPoint (Collision|BreakHitResult _outhit)) (Transformation|GetActorLocation _asbp_tile)))) (Math|Float|Absolute(Float) (.y (- (.ImpactPoint (Collision|BreakHitResult _outhit)) (Transformation|GetActorLocation _asbp_tile))))) false true) (Math|Vector|MakeVector 0.0 (* (Math|Float|Sign(Float) (.y (- (.ImpactPoint (Collision|BreakHitResult _outhit)) (Transformation|GetActorLocation _asbp_tile)))) _returnvalue) 5e+01) (Math|Vector|MakeVector (* (Math|Float|Sign(Float) (.x (- (.ImpactPoint (Collision|BreakHitResult _outhit)) (Transformation|GetActorLocation _asbp_tile)))) _returnvalue) 0.0 5e+01))) "0, 0, 0" "1.000000,1.000000,1.000000") "Undefined" "MultiplyWithRoot" 0 (select (> (Math|Float|Absolute(Float) (.x (- (.ImpactPoint (Collision|BreakHitResult _outhit)) (Transformation|GetActorLocation _asbp_tile)))) (Math|Float|Absolute(Float) (.y (- (.ImpactPoint (Collision|BreakHitResult _outhit)) (Transformation|GetActorLocation _asbp_tile))))) false true) (Variables|/Game/02_Blueprint/01_Core/BP_GameBoard.BP_GameBoard_C|GetWallLengthInUnits (Variables|Default|GetGameBoard_Ref)) 0)
            (Default|DecrementWallCountforCurrentPlayer _gamestate_ref_2)
            (Utilities|Array|Add (Variables|/Game/02_Blueprint/01_Core/GS_Quoridor.GS_Quoridor_C|GetPlacedWalls _gamestate_ref_2) (Utilities|Struct|MakeS_WallData (Utilities|Struct|MakeIntPoint (Variables|/Game/02_Blueprint/01_Core/BP_Tile.BP_Tile_C|GetGridX _asbp_tile) (Variables|/Game/02_Blueprint/01_Core/BP_Tile.BP_Tile_C|GetGridY _asbp_tile)) (select (> (Math|Float|Absolute(Float) (.x (- (.ImpactPoint (Collision|BreakHitResult _outhit)) (Transformation|GetActorLocation _asbp_tile)))) (Math|Float|Absolute(Float) (.y (- (.ImpactPoint (Collision|BreakHitResult _outhit)) (Transformation|GetActorLocation _asbp_tile))))) false true) (> (select (select (> (Math|Float|Absolute(Float) (.x (- (.ImpactPoint (Collision|BreakHitResult _outhit)) (Transformation|GetActorLocation _asbp_tile)))) (Math|Float|Absolute(Float) (.y (- (.ImpactPoint (Collision|BreakHitResult _outhit)) (Transformation|GetActorLocation _asbp_tile))))) false true) (Math|Float|Sign(Float) (.y (- (.ImpactPoint (Collision|BreakHitResult _outhit)) (Transformation|GetActorLocation _asbp_tile)))) (Math|Float|Sign(Float) (.x (- (.ImpactPoint (Collision|BreakHitResult _outhit)) (Transformation|GetActorLocation _asbp_tile))))) 0.0)))
            (Default|ToggleTurn _gamestate_ref_2)))))))

(event Input|MouseEvents|LeftMouseButton
  (params (Key :type Key%20Structure :default "None"))
  (bind _hitresult (Game|Player|GetHitResultUnderCursorbyChannel "TraceTypeQuery1" true))
  (bind _gamestate_ref (Variables|Default|GetGameState_Ref))
  (bind _gamestate_ref_2 (Variables|Default|GetGameState_Ref))
  (bind _gamestate_ref_3 (Variables|Default|GetGameState_Ref))
  (bind _gamestate_ref_4 (Variables|Default|GetGameState_Ref))
  (bind _gameboard_ref (Variables|Default|GetGameBoard_Ref))
  (bind _location (Collision|BreakHitResult _hitresult))
  (bind _bisplayeroneturn (Variables|/Game/02_Blueprint/01_Core/GS_Quoridor.GS_Quoridor_C|GetbIsPlayerOneTurn _gamestate_ref_3))
  (bind _gridspacing (Variables|/Game/02_Blueprint/01_Core/BP_GameBoard.BP_GameBoard_C|GetGridSpacing _gameboard_ref))
  (bind _returnvalue (/ _gridspacing 2.0))
  ;[0.15 0.15 0.15 0.5] Inputs
  (:Released
    ;;[0.15 0.15 0.15 0.5] TurnControl
    (bind _bcaninteract (CallFunction|CanInteract))
    (if _bcaninteract
      (bind (_outhit _returnvalue_2) (Collision|LineTraceByChannel _location (+ _location "0.000000,0.000000,-5000.000000") "TraceTypeQuery1" false 0 "None"))
      (if _returnvalue_2
        (bind _asbp_tile (Utilities|Casting|CastToBP_Tile (.HitActor (Collision|BreakHitResult _outhit))))
        (switch Utilities|FlowControl|Switch|SwitchonE_ActionState (Variables|Default|GeteCurrentActionState)
          (:NewEnumerator0
            ;[0.15 0.15 0.15 0.5] Move Pawn
            (Default|AttemptMoveto (select (Variables|/Game/02_Blueprint/01_Core/GS_Quoridor.GS_Quoridor_C|GetbIsPlayerOneTurn _gamestate_ref_4) (Variables|/Game/02_Blueprint/01_Core/GS_Quoridor.GS_Quoridor_C|GetPlayerOnePawn _gamestate_ref_4) (Variables|/Game/02_Blueprint/01_Core/GS_Quoridor.GS_Quoridor_C|GetPlayerTwoPawn _gamestate_ref_4)) (Utilities|Struct|MakeIntPoint (Variables|/Game/02_Blueprint/01_Core/BP_Tile.BP_Tile_C|GetGridX _asbp_tile) (Variables|/Game/02_Blueprint/01_Core/BP_Tile.BP_Tile_C|GetGridY _asbp_tile)) (Math|Vector|MakeVector (.x (Transformation|GetActorLocation _asbp_tile)) (.y (Transformation|GetActorLocation _asbp_tile)) (Variables|/Game/02_Blueprint/01_Core/BP_GameBoard.BP_GameBoard_C|GetPawnSpawnHeight (Variables|Default|GetGameBoard_Ref))))
            (bind _bgamehasbeenwon (Default|CheckforWinCondition _gamestate_ref_3 _bisplayeroneturn))
            (if _bgamehasbeenwon
              ;;[0.15 0.15 0.15 0.5] EndGame
              (bind _returnvalue_3 (UserInterface|CreateWidget "/Game/02_Blueprint/03_UI/WBP_EndGame.WBP_EndGame_C" 0 (|GenerictoText (select _bisplayeroneturn "Oyuncu 1 Kazandı!" "Oyuncu 2 Kazandı!"))))
              (UserInterface|Viewport|AddtoViewport _returnvalue_3 0)
              (Variables|Default|SetbShowMouseCursor true)
              (Input|SetInputModeUIOnly self _returnvalue_3 "DoNotLock" false)))
          (:NewEnumerator1
            ;[0.15 0.15 0.15 0.5] MoveWall
            (if (> (select (Variables|/Game/02_Blueprint/01_Core/GS_Quoridor.GS_Quoridor_C|GetbIsPlayerOneTurn _gamestate_ref) (Variables|/Game/02_Blueprint/01_Core/GS_Quoridor.GS_Quoridor_C|GetPlayerOneWallCount _gamestate_ref) (Variables|/Game/02_Blueprint/01_Core/GS_Quoridor.GS_Quoridor_C|GetPlayerTwoWallCount _gamestate_ref)) 0)
              (Game|SpawnActorfromClass "/Game/02_Blueprint/01_Core/BP_Wall.BP_Wall_C" (Math|Transform|MakeTransform (+ (Transformation|GetActorLocation _asbp_tile) (select (select (> (Math|Float|Absolute(Float) (.x (- (.ImpactPoint (Collision|BreakHitResult _outhit)) (Transformation|GetActorLocation _asbp_tile)))) (Math|Float|Absolute(Float) (.y (- (.ImpactPoint (Collision|BreakHitResult _outhit)) (Transformation|GetActorLocation _asbp_tile))))) false true) (Math|Vector|MakeVector 0.0 (* (Math|Float|Sign(Float) (.y (- (.ImpactPoint (Collision|BreakHitResult _outhit)) (Transformation|GetActorLocation _asbp_tile)))) _returnvalue) 5e+01) (Math|Vector|MakeVector (* (Math|Float|Sign(Float) (.x (- (.ImpactPoint (Collision|BreakHitResult _outhit)) (Transformation|GetActorLocation _asbp_tile)))) _returnvalue) 0.0 5e+01))) "0, 0, 0" "1.000000,1.000000,1.000000") "Undefined" "MultiplyWithRoot" 0 (select (> (Math|Float|Absolute(Float) (.x (- (.ImpactPoint (Collision|BreakHitResult _outhit)) (Transformation|GetActorLocation _asbp_tile)))) (Math|Float|Absolute(Float) (.y (- (.ImpactPoint (Collision|BreakHitResult _outhit)) (Transformation|GetActorLocation _asbp_tile))))) false true) (Variables|/Game/02_Blueprint/01_Core/BP_GameBoard.BP_GameBoard_C|GetWallLengthInUnits (Variables|Default|GetGameBoard_Ref)) 0)
              (Default|DecrementWallCountforCurrentPlayer _gamestate_ref_2)
              (Utilities|Array|Add (Variables|/Game/02_Blueprint/01_Core/GS_Quoridor.GS_Quoridor_C|GetPlacedWalls _gamestate_ref_2) (Utilities|Struct|MakeS_WallData (Utilities|Struct|MakeIntPoint (Variables|/Game/02_Blueprint/01_Core/BP_Tile.BP_Tile_C|GetGridX _asbp_tile) (Variables|/Game/02_Blueprint/01_Core/BP_Tile.BP_Tile_C|GetGridY _asbp_tile)) (select (> (Math|Float|Absolute(Float) (.x (- (.ImpactPoint (Collision|BreakHitResult _outhit)) (Transformation|GetActorLocation _asbp_tile)))) (Math|Float|Absolute(Float) (.y (- (.ImpactPoint (Collision|BreakHitResult _outhit)) (Transformation|GetActorLocation _asbp_tile))))) false true) (> (select (select (> (Math|Float|Absolute(Float) (.x (- (.ImpactPoint (Collision|BreakHitResult _outhit)) (Transformation|GetActorLocation _asbp_tile)))) (Math|Float|Absolute(Float) (.y (- (.ImpactPoint (Collision|BreakHitResult _outhit)) (Transformation|GetActorLocation _asbp_tile))))) false true) (Math|Float|Sign(Float) (.y (- (.ImpactPoint (Collision|BreakHitResult _outhit)) (Transformation|GetActorLocation _asbp_tile)))) (Math|Float|Sign(Float) (.x (- (.ImpactPoint (Collision|BreakHitResult _outhit)) (Transformation|GetActorLocation _asbp_tile))))) 0.0)))
              (Default|ToggleTurn _gamestate_ref_2))))))))

(fn ConstructionScript)

(fn FindOffset
  (params (X :type Float%20%28double-precision%29) (Y :type Float%20%28double-precision%29) (bIs%20horizantal :type Boolean))
  (bind _gameboard_ref (Variables|Default|GetGameBoard_Ref))
  (bind _gridspacing (Variables|/Game/02_Blueprint/01_Core/BP_GameBoard.BP_GameBoard_C|GetGridSpacing _gameboard_ref))
  (bind _returnvalue (/ _gridspacing 2.0))
  (return (select bIs%20horizantal (Math|Vector|MakeVector (* (Math|Float|Sign(Float) X) _returnvalue) 0.0 5e+01) (Math|Vector|MakeVector 0.0 (* (Math|Float|Sign(Float) Y) _returnvalue) 5e+01))))

(fn IsValidPawnMove
  (params (CurrentLocation :type Int%20Point%20Structure) (TargetLocation :type Int%20Point%20Structure))
  (bind (_x _y) (Utilities|Struct|BreakIntPoint TargetLocation))
  (bind (_x_2 _y_2) (Utilities|Struct|BreakIntPoint CurrentLocation))
  (bind (_x_3 _y_3) (Utilities|Struct|BreakIntPoint CurrentLocation))
  (bind (_x_4 _y_4) (Utilities|Struct|BreakIntPoint CurrentLocation))
  (bind (_x_5 _y_5) (Utilities|Struct|BreakIntPoint TargetLocation))
  (bind _returnvalue (+ CurrentLocation TargetLocation))
  (bind _gamestate_ref (Variables|Default|GetGameState_Ref))
  (bind _intpoint (Utilities|Struct|MakeIntPoint _x_4 _y_5))
  (bind _intpoint_2 (Utilities|Struct|MakeIntPoint _x_5 _y_4))
  (bind _returnvalue_2 (- _x _x_2))
  (bind _returnvalue_3 (- _y _y_2))
  (bind _bisplayeroneturn (Variables|/Game/02_Blueprint/01_Core/GS_Quoridor.GS_Quoridor_C|GetbIsPlayerOneTurn _gamestate_ref))
  (bind _playeronegridlocation (Variables|/Game/02_Blueprint/01_Core/GS_Quoridor.GS_Quoridor_C|GetPlayerOneGridLocation _gamestate_ref))
  (bind _playertwogridlocation (Variables|/Game/02_Blueprint/01_Core/GS_Quoridor.GS_Quoridor_C|GetPlayerTwoGridLocation _gamestate_ref))
  (bind (_x_6 _y_6) (Utilities|Struct|BreakIntPoint _intpoint))
  (bind (_x_7 _y_7) (Utilities|Struct|BreakIntPoint _intpoint_2))
  (bind _returnvalue_4 (Math|Integer|Absolute(Integer) _returnvalue_3))
  (bind _returnvalue_5 (Math|Integer|Absolute(Integer) _returnvalue_2))
  (bind _returnvalue_6 (select _bisplayeroneturn _playertwogridlocation _playeronegridlocation))
  (bind (_x_8 _y_8) (Utilities|Struct|BreakIntPoint _returnvalue_6))
  (bind (_x_9 _y_9) (Utilities|Struct|BreakIntPoint _returnvalue_6))
  (bind (_x_10 _y_10) (Utilities|Struct|BreakIntPoint _returnvalue_6))
  (switch int (+ _returnvalue_5 _returnvalue_4)
    (:Default
      (return false))
    (:1
      (return true))
    (:2
      (if (or (== _returnvalue_5 2) (== _returnvalue_4 2)) ; Branch 1
        (if (and (== (/ (.x _returnvalue) 2) _x_8) (== (/ (.y _returnvalue) 2) _y_8)) ; Branch 2
          (return true)
          (else
            (return false)))
        (elif (or (and (== _x_9 _x_6) (== _y_9 _y_6)) (and (== _x_9 _x_7) (== _y_9 _y_7))) ; Branch 3
          (if (Default|IsPathBlockedbyWall (Variables|Default|GetGameState_Ref) _returnvalue_6 (Utilities|Struct|MakeIntPoint (- (* _x_10 2) _x_3) (- (* _y_10 2) _y_3))) ; Branch 4
            (return true)
            (else
              (return false)))
          (else
            (return false)))))))

(fn CanInteract
  (bind _gamestate_ref (Variables|Default|GetGameState_Ref))
  (bind _bisplayeroneturn (Variables|/Game/02_Blueprint/01_Core/GS_Quoridor.GS_Quoridor_C|GetbIsPlayerOneTurn _gamestate_ref))
  (Utilities|IsValid (Variables|Default|GetGameState_Ref)
    (:Is%20Valid
      (bind _asgi_quoridor (Utilities|Casting|CastToGI_Quoridor (Game|GetGameInstance)))
      (Development|PrintString (Utilities|String|ToString(Boolean) _bisplayeroneturn))
      (return (or (Utilities|Enum|Equal(Enum) (Variables|/Game/02_Blueprint/01_Core/GI_Quoridor.GI_Quoridor_C|GetSelectedGameMode _asgi_quoridor) "NewEnumerator0") (and (not (Utilities|Enum|Equal(Enum) (Variables|/Game/02_Blueprint/01_Core/GI_Quoridor.GI_Quoridor_C|GetSelectedGameMode _asgi_quoridor) "NewEnumerator0")) _bisplayeroneturn))))
    (:Is%20Not%20Valid
      (return false))))