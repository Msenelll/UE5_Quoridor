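; Player pawn for a Quoridor game that handles moves and wall placement for whichever player's turn it is.
; Moves allow single steps, straight jumps over the opponent and wall-forced diagonals, then GS_Quoridor checks walls, stores position and toggles turn.
; Walls spawn as BP_Wall using BP_GameBoard spacing, with collision rejecting overlaps.
; Successful walls are recorded and decrement the count; a failed spawn still passes the turn.
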(event EventBeginPlay
  (bind _asgs_quoridor (Utilities|Casting|CastToGS_Quoridor (Game|GetGameState)))
  (Variables|Default|SetGameState_Ref _asgs_quoridor)
  (bind _returnvalue (Actor|GetActorOfClass "/Game/02_Blueprint/01_Core/BP_GameBoard.BP_GameBoard_C"))
  (Variables|Default|SetGameBoard_Ref _returnvalue))

(event Collision|EventActorBeginOverlap
  (params (OtherActor :type Actor%20Object%20Reference)))

(event EventTick
  (params (DeltaSeconds :type Float%20%28single-precision%29)))

(fn ConstructionScript)

(fn AttemptMoveto
  (params (TargetGridLocation :type Int%20Point%20Structure) (TargetWorldLocation :type Vector))
  (bind _gamestate_ref (Variables|Default|GetGameState_Ref))
  (bind _gamestate_ref_2 (Variables|Default|GetGameState_Ref))
  (bind _bisplayeroneturn (Variables|/Game/02_Blueprint/01_Core/GS_Quoridor.GS_Quoridor_C|GetbIsPlayerOneTurn _gamestate_ref_2))
  (bind _playertwogridlocation (Variables|/Game/02_Blueprint/01_Core/GS_Quoridor.GS_Quoridor_C|GetPlayerTwoGridLocation _gamestate_ref_2))
  (bind _playeronegridlocation (Variables|/Game/02_Blueprint/01_Core/GS_Quoridor.GS_Quoridor_C|GetPlayerOneGridLocation _gamestate_ref_2))
  (bind _returnvalue (select _bisplayeroneturn _playeronegridlocation _playertwogridlocation))
  (if (CallFunction|IsValidPawnMove _returnvalue TargetGridLocation) ; A
    (if (not (Default|IsPathBlockedbyWall _gamestate_ref_2 _returnvalue TargetGridLocation (Utilities|Struct|MakeS_WallData TargetGridLocation false false))) ; B
      (Transformation|SetActorLocation TargetWorldLocation false false)
      (Default|UpdateCurrentPlayerGridLocation _gamestate_ref TargetGridLocation)
      (Default|ToggleTurn _gamestate_ref)
      (return true)
      (else
        _)))
  (return false))

(fn IsValidPawnMove
  (params (CurrentLocation :type Int%20Point%20Structure) (TargetLocation :type Int%20Point%20Structure))
  (bind (_x _y) (Utilities|Struct|BreakIntPoint TargetLocation))
  (bind (_x_2 _y_2) (Utilities|Struct|BreakIntPoint CurrentLocation))
  (bind (_x_3 _y_3) (Utilities|Struct|BreakIntPoint CurrentLocation))
  (bind (_x_4 _y_4) (Utilities|Struct|BreakIntPoint CurrentLocation))
  (bind (_x_5 _y_5) (Utilities|Struct|BreakIntPoint TargetLocation))
  (bind _returnvalue (+ CurrentLocation TargetLocation))
  (bind _gamestate_ref (Variables|Default|GetGameState_Ref))
  (bind _intpoint (Utilities|Struct|MakeIntPoint _x_4 _y_5))
  (bind _intpoint_2 (Utilities|Struct|MakeIntPoint _x_5 _y_4))
  (bind _returnvalue_2 (- _x _x_2))
  (bind _returnvalue_3 (- _y _y_2))
  (bind _bisplayeroneturn (Variables|/Game/02_Blueprint/01_Core/GS_Quoridor.GS_Quoridor_C|GetbIsPlayerOneTurn _gamestate_ref))
  (bind _playeronegridlocation (Variables|/Game/02_Blueprint/01_Core/GS_Quoridor.GS_Quoridor_C|GetPlayerOneGridLocation _gamestate_ref))
  (bind _playertwogridlocation (Variables|/Game/02_Blueprint/01_Core/GS_Quoridor.GS_Quoridor_C|GetPlayerTwoGridLocation _gamestate_ref))
  (bind (_x_6 _y_6) (Utilities|Struct|BreakIntPoint _intpoint))
  (bind (_x_7 _y_7) (Utilities|Struct|BreakIntPoint _intpoint_2))
  (bind _returnvalue_4 (Math|Integer|Absolute(Integer) _returnvalue_3))
  (bind _returnvalue_5 (Math|Integer|Absolute(Integer) _returnvalue_2))
  (bind _returnvalue_6 (select _bisplayeroneturn _playertwogridlocation _playeronegridlocation))
  (bind (_x_8 _y_8) (Utilities|Struct|BreakIntPoint _returnvalue_6))
  (bind (_x_9 _y_9) (Utilities|Struct|BreakIntPoint _returnvalue_6))
  (bind (_x_10 _y_10) (Utilities|Struct|BreakIntPoint _returnvalue_6))
  (switch int (+ _returnvalue_5 _returnvalue_4)
    (:Default
      (return false))
    (:1
      (return true))
    (:2
      (if (or (== _returnvalue_5 2) (== _returnvalue_4 2)) ; Branch 1
        (if (and (== (/ (.x _returnvalue) 2) _x_8) (== (/ (.y _returnvalue) 2) _y_8)) ; Branch 2
          (return true)
          (else
            (return false)))
        (elif (or (and (== _x_9 _x_6) (== _y_9 _y_6)) (and (== _x_9 _x_7) (== _y_9 _y_7))) ; Branch 3
          (if (Default|IsPathBlockedbyWall (Variables|Default|GetGameState_Ref) _returnvalue_6 (Utilities|Struct|MakeIntPoint (- (* _x_10 2) _x_3) (- (* _y_10 2) _y_3))) ; Branch 4
            (return true)
            (else
              (return false)))
          (else
            (return false)))))))

(fn AttemptPlaceWall
  (params (TargetGridLocation :type Int%20Point%20Structure) (bIsHorizontal :type Boolean) (bIsPositiveOffset :type Boolean))
  (bind (_x _y) (Utilities|Struct|BreakIntPoint TargetGridLocation))
  (bind _gameboard_ref (Variables|Default|GetGameBoard_Ref))
  (bind _gamestate_ref (Variables|Default|GetGameState_Ref))
  (bind _gamestate_ref_2 (Variables|Default|GetGameState_Ref))
  (bind _gridspacing (Variables|/Game/02_Blueprint/01_Core/BP_GameBoard.BP_GameBoard_C|GetGridSpacing _gameboard_ref))
  (bind _returnvalue (/ _gridspacing 2.0))
  (if (Utilities|IsValid (Variables|Default|GetGameBoard_Ref))
    (if (> (select (Variables|/Game/02_Blueprint/01_Core/GS_Quoridor.GS_Quoridor_C|GetbIsPlayerOneTurn _gamestate_ref) (Variables|/Game/02_Blueprint/01_Core/GS_Quoridor.GS_Quoridor_C|GetPlayerOneWallCount _gamestate_ref) (Variables|/Game/02_Blueprint/01_Core/GS_Quoridor.GS_Quoridor_C|GetPlayerTwoWallCount _gamestate_ref)) 0)
      (bind _returnvalue_2 (Game|SpawnActorfromClass "/Game/02_Blueprint/01_Core/BP_Wall.BP_Wall_C" (Math|Transform|MakeTransform (Math|Vector|MakeVector (+ (* _x _gridspacing) (* (select bIsHorizontal 0.0 _returnvalue) (select bIsPositiveOffset 1.0 -1.0))) (+ (* _y _gridspacing) (* (select bIsHorizontal _returnvalue 0.0) (select bIsPositiveOffset 1.0 -1.0))) (+ (Variables|/Game/02_Blueprint/01_Core/BP_GameBoard.BP_GameBoard_C|GetPawnSpawnHeight _gameboard_ref) 75.0)) "0, 0, 0" "1.000000,1.000000,1.000000") "DontSpawnIfColliding" "MultiplyWithRoot" 0 bIsHorizontal (Variables|/Game/02_Blueprint/01_Core/BP_GameBoard.BP_GameBoard_C|GetWallLengthInUnits _gameboard_ref) 0))
      (Utilities|IsValid _returnvalue_2
        (:Is%20Valid
          (Utilities|Array|Add (Variables|/Game/02_Blueprint/01_Core/GS_Quoridor.GS_Quoridor_C|GetPlacedWalls _gamestate_ref_2) (Utilities|Struct|MakeS_WallData TargetGridLocation bIsHorizontal bIsPositiveOffset))
          (Default|DecrementWallCountforCurrentPlayer _gamestate_ref_2)
          (Default|ToggleTurn _gamestate_ref_2)
          (return true))
        (:Is%20Not%20Valid
          (Default|ToggleTurn _gamestate_ref_2)
          (return false))))))