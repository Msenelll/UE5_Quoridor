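; Game mode for Quoridor that sets up both player pawns when play begins.
; It moves player 0's existing pawn to a fixed start position and registers it as player one in GS_Quoridor.
; It then spawns a second, unpossessed BP_PlayerPawn at another fixed position, changes its mesh material and registers it as player two.
; Positions are hardcoded, as the board location lookup is left unconnected.
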(event EventBeginPlay
  (bind _returnvalue (Game|Player|GetPlayerPawn 0))
  (bind _asgs_quoridor (Utilities|Casting|CastToGS_Quoridor (Game|GetGameState)))
  ;[0.15 0.15 0.15 0.5] Create Player Pawn
  (bind _output_get (Variables|Default|SetRef_GS _asgs_quoridor))
  (Variables|/Game/02_Blueprint/01_Core/GS_Quoridor.GS_Quoridor_C|SetPlayerOnePawn _output_get 0)
  (Transformation|SetActorLocation _returnvalue "800.000000,0.000000,150.000000" false false)
  (bind _asbp_player_pawn (Utilities|Casting|CastToBP_PlayerPawn _returnvalue))
  (Variables|/Game/02_Blueprint/01_Core/GS_Quoridor.GS_Quoridor_C|SetPlayerOnePawn _output_get _asbp_player_pawn)
  ;[0.15 0.15 0.15 0.5] Create Player 2 Pawn
  (bind _returnvalue_2 (Game|SpawnActorfromClass "/Game/02_Blueprint/02_Pawns/BP_PlayerPawn.BP_PlayerPawn_C" (Math|Transform|MakeTransform "800.000000,1600.000000,150.000000" "0, 0, 0" "1.000000,1.000000,1.000000") "Undefined" "MultiplyWithRoot" 0 0))
  (Rendering|Material|SetMaterial (Actor|GetComponentbyClass _returnvalue_2 "/Script/Engine.StaticMeshComponent") 0 "/Engine/EngineDebugMaterials/MAT_LevelColorationLitLightmapUV.MAT_LevelColorationLitLightmapUV")
  (Variables|/Game/02_Blueprint/01_Core/GS_Quoridor.GS_Quoridor_C|SetPlayerTwoPawn _output_get _returnvalue_2))

(event EventTick
  (params (DeltaSeconds :type Float%20%28single-precision%29)))

(fn ConstructionScript)