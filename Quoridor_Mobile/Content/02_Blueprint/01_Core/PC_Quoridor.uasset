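; Player controller for a Quoridor game that moves the controlled BP_PlayerPawn to the clicked spot.
; On BeginPlay it switches the view to a CameraActor in the level, shows the cursor and sets game-only input.
; Left mouse release, or the actor touch-begin event, traces straight down from the cursor hit point.
; A hit prints that actor's location and teleports the pawn to the hit XY at a fixed height, without move validation.
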(event EventTick
  (params (DeltaSeconds :type Float%20%28single-precision%29)))

(event EventBeginPlay
  ;[0.15 0.15 0.15 0.5] Preset
  (bind _returnvalue (Actor|GetActorOfClass "/Script/Engine.CameraActor"))
  (Game|Player|SetViewTargetwithBlend _returnvalue 0.0 "VTBlend_Linear" 0.0 false)
  (Variables|Default|SetbShowMouseCursor true)
  (Input|SetInputModeGameOnly self false))

(event EventActorOnInputTouchBegin
  (params (FingerIndex :type ETouchIndex%20Enum :default "Touch1"))
  (bind _hitresult (Game|Player|GetHitResultUnderCursorbyChannel "TraceTypeQuery1" true))
  (bind _location (Collision|BreakHitResult _hitresult))
  ;[0.15 0.15 0.15 0.5] Inputs
  (bind (_outhit _returnvalue) (Collision|LineTraceByChannel _location (+ _location "0.000000,0.000000,-5000.000000") "TraceTypeQuery1" false 0 "None"))
  (if _returnvalue
    (Development|PrintString (Utilities|String|ToString(Vector) (Transformation|GetActorLocation (.HitActor (Collision|BreakHitResult _outhit)))))
    (bind _asbp_player_pawn (Utilities|Casting|CastToBP_PlayerPawn (Pawn|GetControlledPawn)))
    (Transformation|SetActorLocation _asbp_player_pawn (+ (* (.Location (Collision|BreakHitResult _outhit)) "1.000000,1.000000,0.000000") "0.000000,0.000000,150.000000") false false)))

(event Input|MouseEvents|LeftMouseButton
  (params (Key :type Key%20Structure :default "None"))
  (bind _hitresult (Game|Player|GetHitResultUnderCursorbyChannel "TraceTypeQuery1" true))
  (bind _location (Collision|BreakHitResult _hitresult))
  ;[0.15 0.15 0.15 0.5] Inputs
  (:Released
    (bind (_outhit _returnvalue) (Collision|LineTraceByChannel _location (+ _location "0.000000,0.000000,-5000.000000") "TraceTypeQuery1" false 0 "None"))
    (if _returnvalue
      (Development|PrintString (Utilities|String|ToString(Vector) (Transformation|GetActorLocation (.HitActor (Collision|BreakHitResult _outhit)))))
      (bind _asbp_player_pawn (Utilities|Casting|CastToBP_PlayerPawn (Pawn|GetControlledPawn)))
      (Transformation|SetActorLocation _asbp_player_pawn (+ (* (.Location (Collision|BreakHitResult _outhit)) "1.000000,1.000000,0.000000") "0.000000,0.000000,150.000000") false false))))

(fn ConstructionScript)