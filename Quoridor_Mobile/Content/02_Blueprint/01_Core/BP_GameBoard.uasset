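; BP_GameBoard is an actor that builds a square grid of cube tiles as a game board when play begins.
; Nested loops spawn a StaticMeshActor per cell at 100-unit spacing, offset from the board's X and Y location.
; Each tile gets a cube mesh and a shared material instance.
; BPGameBoardLoc is overwritten with every cell position at zero height, so it ends holding the last one.
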(event EventBeginPlay
  (bind _returnvalue (Transformation|GetActorLocation))
  ;[0.15 0.15 0.15 0.5] Create a GameBoard
  (for _index (range 0 9)
    (for _index_2 (range 0 9)
      (bind _returnvalue_2 (Game|SpawnActorfromClass "/Script/Engine.StaticMeshActor" (Math|Transform|MakeTransform (Math|Vector|MakeVector (+ (Math|Conversions|ToFloat(Integer) (* _index_2 100)) (.x _returnvalue)) (+ (Math|Conversions|ToFloat(Integer) (* _index 100)) (.y _returnvalue)) 0.0) "0, 0, 0" "1.000000,1.000000,1.000000") "Undefined" "MultiplyWithRoot" 0 0))
      (Components|StaticMesh|SetStaticMesh (Variables|/Script/Engine.StaticMeshActor|GetStaticMeshComponent _returnvalue_2) "/Engine/EngineMeshes/Cube.Cube")
      (Rendering|Material|SetMaterial (Variables|/Script/Engine.StaticMeshActor|GetStaticMeshComponent _returnvalue_2) 0 "/Engine/BasicShapes/BasicShapeMaterial_Inst.BasicShapeMaterial_Inst")
      (Variables|Default|SetBP_GameBoard_Loc (Math|Vector|MakeVector (+ (Math|Conversions|ToFloat(Integer) (* _index_2 100)) (.x _returnvalue)) (+ (Math|Conversions|ToFloat(Integer) (* _index 100)) (.y _returnvalue)) 0.0)))))

(event Collision|EventActorBeginOverlap
  (params (OtherActor :type Actor%20Object%20Reference)))

(event EventTick
  (params (DeltaSeconds :type Float%20%28single-precision%29)))

(fn ConstructionScript)